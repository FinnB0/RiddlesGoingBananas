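; BPC_ColorUsage is a component that switches one color channel on and off, draining a limited usage budget while active.
; Toggling on requires remaining Time and starts a looping one-second timer, apparently driving Usage_Tick, which lowers Time and deactivates the channel at zero.
; Each switch calls a dispatcher and writes the state to the MPC_RGB material parameter collection, using the channel's enum name as the parameter.
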(event Custom|ActivateColorUseage
  (bind _returnvalue (Utilities|Time|SetTimerbyEvent (EventDispatchers|CreateEvent :!event Custom|Usage_Tick) 1.0 true))
  (Variables|Default|SetUsageTimer _returnvalue)
  (Variables|Default|SetbIsUsed true)
  (Default|CallDPToggleColorUsage true)
  (Rendering|Material|SetScalarParameterValue "/Game/Materials/MPC_RGB.MPC_RGB" (Utilities|String|StringToName (Utilities|String|EnumtoString (Variables|Default|GetE_ColorChannel))) (Math|Conversions|ToFloat(Boolean) (Variables|Default|GetbIsUsed)) :!class /Script/Engine.KismetMaterialLibrary))

(event Custom|DeactivateColorUsage
  (Utilities|Time|PauseTimerbyHandle (Variables|Default|GetUsageTimer))
  (Variables|Default|SetbIsUsed false)
  (Default|CallDPToggleColorUsage false)
  (Rendering|Material|SetScalarParameterValue "/Game/Materials/MPC_RGB.MPC_RGB" (Utilities|String|StringToName (Utilities|String|EnumtoString (Variables|Default|GetE_ColorChannel))) (Math|Conversions|ToFloat(Boolean) (Variables|Default|GetbIsUsed)) :!class /Script/Engine.KismetMaterialLibrary))

(event Custom|Usage_Tick
  (bind _output_get (Variables|Default|SetTime (- (Variables|Default|GetTime) 5.0)))
  (if (<= (Math|Float|Clamp(Float) _output_get 0.0 255.0) 0.0)
    (CallFunction|DeactivateColorUsage)))

(event Custom|ToggleUsage
  (if (Variables|Default|GetbIsUsed)
    (CallFunction|DeactivateColorUsage)
    (elif (> (Variables|Default|GetTime) 0.0)
      (CallFunction|ActivateColorUseage))))