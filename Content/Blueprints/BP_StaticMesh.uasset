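; BP_StaticMesh is a colored mesh actor that becomes visible and solid, or hidden and non-colliding, based on RGB channel input.
; The construction script creates a dynamic instance of MM_GridSurface and sets its SurfaceColor from the actor's Color.
; CheckChannels shows the actor when any positive input channel matches a nonzero channel in Color, otherwise hides it, printing the result for debugging.
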(event EventCheckChannels
  (params (R :type Float%20%28double-precision%29) (G :type Float%20%28double-precision%29) (B :type Float%20%28double-precision%29))
  (if (or (or (and (> R 0.0) (!= (.r (Variables|Default|GetColor)) 0.0)) (and (> G 0.0) (!= (.g (Variables|Default|GetColor)) 0.0))) (and (> B 0.0) (!= (.b (Variables|Default|GetColor)) 0.0)))
    (Development|PrintString "Visible")
    (Collision|SetActorEnableCollision true)
    (Rendering|SetActorHiddenInGame false)
    (else
      (Development|PrintString "Hidden")
      (Collision|SetActorEnableCollision false)
      (Rendering|SetActorHiddenInGame true))))

(fn ConstructionScript
  (bind _returnvalue (Rendering|Material|CreateDynamicMaterialInstance (Variables|Debug|GetStaticMeshComponent) 0 "/Game/Materials/MM_GridSurface.MM_GridSurface" "None" :!class /Script/Engine.PrimitiveComponent))
  (Rendering|Material|SetVectorParameterValue _returnvalue "SurfaceColor" (Variables|Default|GetColor) :!class /Script/Engine.MaterialInstanceDynamic))