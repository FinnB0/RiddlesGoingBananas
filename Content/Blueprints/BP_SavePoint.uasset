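; BP_SavePoint is a save point actor that toggles the player pawn's color usage message pause while the player overlaps it.
; Begin and end overlap events check for player pawn 0 and call PauseColorUsageMessage with true on entry and false on exit.
; The graph contains no save logic, and its construction script is empty.
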(event Collision|EventActorBeginOverlap
  (params (OtherActor :type Actor%20Object%20Reference))
  (if (== OtherActor (Game|Player|GetPlayerPawn 0))
    (Class|BPIPlayerPawn|PauseColorUsage(Message) (Game|Player|GetPlayerPawn 0) true)))

(event Collision|EventActorEndOverlap
  (params (OtherActor :type Actor%20Object%20Reference))
  (if (== OtherActor (Game|Player|GetPlayerPawn 0))
    (Class|BPIPlayerPawn|PauseColorUsage(Message) (Game|Player|GetPlayerPawn 0) false)))

(fn ConstructionScript)